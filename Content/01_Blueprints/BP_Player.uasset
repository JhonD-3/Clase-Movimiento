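; Player character Blueprint with Enhanced Input movement, look, jump, run and a montage-based melee attack.
; BeginPlay adds the input mapping context; movement follows control yaw, and running switches max walk speed.
; Attacks pick a montage by AttackIndex, gated by CanAttack, with both reset on montage completion.
; HitDetection sphere-traces WorldStatic objects at an index-selected hand or foot socket with debug drawing, but is not called here and ignores results.
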(event Input|EnhancedActionEvents|EnhancedInputActionIA_Run
  (params (ActionValue :type Boolean) (ElapsedSeconds :type Float%20%28double-precision%29) (TriggeredSeconds :type Float%20%28double-precision%29) (InputAction :type Input%20Action%20Object%20Reference :default "/Game/01_Blueprints/01_Player/02_Inputs/IA_Run.IA_Run"))
  (bind _charactermovement (Variables|Character|GetCharacterMovement))
  (:Triggered
    (Variables|/Script/Engine.CharacterMovementComponent|SetMaxWalkSpeed _charactermovement 1.5e+03))
  (:Canceled
    (Variables|/Script/Engine.CharacterMovementComponent|SetMaxWalkSpeed _charactermovement 7.5e+02 :!label _label))
  (:Completed
    (goto _label)))

(event Input|EnhancedActionEvents|EnhancedInputActionIA_Attack
  (params (ActionValue :type Boolean) (ElapsedSeconds :type Float%20%28double-precision%29) (TriggeredSeconds :type Float%20%28double-precision%29) (InputAction :type Input%20Action%20Object%20Reference :default "/Game/01_Blueprints/01_Player/02_Inputs/IA_Attack.IA_Attack"))
  (Variables|Default|GetCanAttack
    (:then
      (Variables|Default|SetCanAttack false)
      (Animation|Montage|PlayMontage (Variables|Character|GetMesh) (Utilities|Select :Index (Variables|Default|GetAttackIndex) :Option%200 "/Game/01_Blueprints/01_Player/01_Animations/Atk1_Boxing_Montage.Atk1_Boxing_Montage" :Option%201 "/Game/01_Blueprints/01_Player/01_Animations/Atk2_Reaction_Montage.Atk2_Reaction_Montage" :Option%202 "/Game/01_Blueprints/01_Player/01_Animations/Atk3_Kick_Montage.Atk3_Kick_Montage")
        (:then
          (Math|Integer|IncrementInt (Variables|Default|GetAttackIndex)))
        (:OnCompleted
          (Variables|Default|SetCanAttack true)
          (Variables|Default|SetAttackIndex 0))))
    (:else)))

(event Input|EnhancedActionEvents|EnhancedInputActionIA_Jump
  (params (ActionValue :type Vector%202D%20Structure) (ElapsedSeconds :type Float%20%28double-precision%29) (TriggeredSeconds :type Float%20%28double-precision%29) (InputAction :type Input%20Action%20Object%20Reference :default "/Game/01_Blueprints/01_Player/02_Inputs/IA_Jump.IA_Jump"))
  (Character|Jump))

(event Input|EnhancedActionEvents|EnhancedInputActionIA_Move
  (params (ActionValue :type Vector%202D%20Structure) (ElapsedSeconds :type Float%20%28double-precision%29) (TriggeredSeconds :type Float%20%28double-precision%29) (InputAction :type Input%20Action%20Object%20Reference :default "/Game/01_Blueprints/01_Player/02_Inputs/IA_Move.IA_Move"))
  (Pawn|Input|AddMovementInput (Math|Vector|GetForwardVector (Math|Rotator|MakeRotator 0.0 0.0 (.yaw (Pawn|GetControlRotation :!class /Script/Engine.Pawn)))) (.y ActionValue) false)
  (Pawn|Input|AddMovementInput (Math|Vector|GetRightVector (Math|Rotator|MakeRotator 0.0 0.0 (.yaw (Pawn|GetControlRotation :!class /Script/Engine.Pawn)))) (.x ActionValue) false))

(event Input|EnhancedActionEvents|EnhancedInputActionIA_Look
  (params (ActionValue :type Vector%202D%20Structure) (ElapsedSeconds :type Float%20%28double-precision%29) (TriggeredSeconds :type Float%20%28double-precision%29) (InputAction :type Input%20Action%20Object%20Reference :default "/Game/01_Blueprints/01_Player/02_Inputs/IA_Look.IA_Look"))
  (Pawn|Input|AddControllerYawInput (.x ActionValue))
  (Pawn|Input|AddControllerPitchInput (.y ActionValue)))

(event EventBeginPlay
  (bind _asplayer_controller (Utilities|Casting|CastToPlayerController (Pawn|GetController)))
  (Utilities|IsValid (PlayerController|LocalPlayerSubsystems|GetEnhancedInputLocalPlayerSubsystem _asplayer_controller)
    (:Is%20Valid
      (Input|AddMappingContext (PlayerController|LocalPlayerSubsystems|GetEnhancedInputLocalPlayerSubsystem _asplayer_controller) "/Game/01_Blueprints/01_Player/02_Inputs/IMC_Player.IMC_Player" 0 "(bIgnoreAllPressedKeysUntilRelease=True,bForceImmediately=False,bNotifyUserSettings=False)"))))

(fn ConstructionScript)

(fn HitDetection
  (bind _mesh (Variables|Character|GetMesh))
  (bind _attackindex (Variables|Default|GetAttackIndex))
  (bind _returnvalue (Utilities|Select :Index _attackindex :Option%200 "LeftHand" :Option%201 "LeftHand" :Option%202 "LeftHand" :Option%203 "LeftFoot"))
  (bind _returnvalue_2 (Transformation|GetSocketLocation _mesh _returnvalue))
  (Collision|SphereTraceForObjects _returnvalue_2 _returnvalue_2 2e+01 (Utilities|Array|MakeArray "ObjectTypeQuery1") false 0 "ForOneFrame"))